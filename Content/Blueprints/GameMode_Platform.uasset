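; GameMode for a local multiplayer platform game that spawns players, plays music and handles player defeat.
; Shortly after BeginPlay, it creates a local player per PlayerStart, then spawns and possesses a BP_Boy_ZD there.
; The first player gets its own Enhanced Input mapping context, while all others share a second one.
; A bound defeat event restarts that player's controller, and a separate RestartGame function reloads the current level.
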(event `self.ReceiveBeginPlay`
  (`|ExecutionSequence`
    (:`then_0`
      (`KismetSystemLibrary.Delay` 0.2)
      (`self.CreatePlayers`))
    (:`then_1`
      (add `self.OnPlayerDefeat` (delegate `PlayerDefeat`)))
    (:`then_2`
      (`GameplayStatics.PlaySound2D` "/Game/Sounds/music.music" 1.0 1.0 0.0 null null))))

(event `PlayerDefeat` :!signature `self.OnPlayerDefeat`
  (params (Boy :type "Character Object Reference"))
  (`self.RestartPlayer` (`Pawn.GetController` Boy)))

(fn `CreatePlayers`
  (bind _returnvalue (`GameplayStatics.GetPlayerController` (`self.Index`)))
  (bind _returnvalue_2 (pcsubsystem `EnhancedInputLocalPlayerSubsystem` (`GameplayStatics.GetPlayerController` (`self.Index`))))
  (bind _outactors (`GameplayStatics.GetAllActorsOfClass` "/Script/Engine.PlayerStart"))
  (for (_array_element _array_index) _outactors
    (bind _output_get (set `self.Index` _array_index))
    (if (== (`self.Index`) 0)
      (`GameplayStatics.CreatePlayer` _output_get)
      (`EnhancedInputSubsystemInterface.AddMappingContext` _returnvalue_2 "/Game/Input/Hero_ZD_Mapping.Hero_ZD_Mapping" 0 (struct))
      (bind _returnvalue_3 (`self.GetTransform` _array_element))
      (bind _returnvalue_4 (`|SpawnActorFromClass` "/Game/Blueprints/Characters/Boy/BP_Boy_ZD.BP_Boy_ZD_C" _returnvalue_3 "Undefined" "MultiplyWithRoot" null null))
      (`Controller.Possess` _returnvalue _returnvalue_4)
      (else
        (`GameplayStatics.CreatePlayer` _output_get)
        (`EnhancedInputSubsystemInterface.AddMappingContext` _returnvalue_2 "/Game/Input/Hero_ZD_Mapping2.Hero_ZD_Mapping2" 0 (struct))
        (bind _returnvalue_5 (`|SpawnActorFromClass` "/Game/Blueprints/Characters/Boy/BP_Boy_ZD.BP_Boy_ZD_C" _returnvalue_3 "Undefined" "MultiplyWithRoot" null null))
        (`Controller.Possess` _returnvalue _returnvalue_5)))))

(fn `RestartGame`
  (bind _returnvalue (`GameplayStatics.GetCurrentLevelName` true))
  (`GameplayStatics.OpenLevel` (`KismetStringLibrary.Conv_StringToName` _returnvalue)))

(fn `UserConstructionScript`)