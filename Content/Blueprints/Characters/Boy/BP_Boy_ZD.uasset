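; Player character for a two-player side-scrolling platformer, moving along X and flipping control rotation to face its direction.
; Jumping adds coyote time and input buffering, and a downward trace while falling toggles collision with platforms.
; Falling onto bats or rats defeats them and bounces the player; other contact defeats the player.
; Defeat removes input, detaches the camera with a shake, then respawns at the controller's tagged start.
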(event `self.ReceiveBeginPlay`
  (`parent.ReceiveBeginPlay`))

(event `self.ReceiveTick`
  (params (DeltaSeconds :type "Float (single-precision)"))
  (`parent.ReceiveTick` DeltaSeconds)
  (`self.UpdateContollerRotation`)
  (`self.Trace for Platforms`)
  (if (and (`self.IsJumpBuffering`) (`self.CanJump`))
    (`self.Jump`)))

(event `EnhancedInput|/Game/Input/Actions/Hero_ZD_Move`
  (params (ActionValue :type "Float (double-precision)") (ElapsedSeconds :type "Float (double-precision)") (TriggeredSeconds :type "Float (double-precision)") (InputAction :type "InputAction Object Reference" :default "/Game/Input/Actions/Hero_ZD_Move.Hero_ZD_Move"))
  (:`Triggered`
    (`self.AddMovementInput` (1.0 0.0 0.0) ActionValue)))

(event `EnhancedInput|/Game/Input/Actions/Hero_ZD_Jump`
  (params (ActionValue :type Boolean) (ElapsedSeconds :type "Float (double-precision)") (TriggeredSeconds :type "Float (double-precision)") (InputAction :type "InputAction Object Reference" :default "/Game/Input/Actions/Hero_ZD_Jump.Hero_ZD_Jump"))
  (:`Started`
    (if (`self.CanJump`)
      (`self.Jump`)
      (bind _asplayer_controller (cast `PlayerController` (`self.GetController`)))
      (`KismetSystemLibrary.PrintString` (`KismetStringLibrary.Conv_IntToString` (`GameplayStatics.GetPlayerControllerID` _asplayer_controller)))
      (else
        (set `self.IsJumpBuffering` true)
        (`KismetSystemLibrary.RetriggerableDelay` (`self.JumpBuffer`))
        (set `self.IsJumpBuffering` false))))
  (:`Canceled`
    (`self.StopJumping`)))

(event `self.Defead`
  (`parent.Defead`)
  (`self.DefeatEffect`))

(event `self.LaunchOnDefeat`
  (`parent.LaunchOnDefeat`)
  (bind _asgame_mode_platform (cast `/Game/Blueprints/GameMode_Platform` (`GameplayStatics.GetGameMode`)))
  (`KismetSystemLibrary.Delay` 2.0)
  (`/Game/Blueprints/GameMode_Platform.OnPlayerDefeat` _asgame_mode_platform self)
  (`self.CallRestartPlayer` self))

(event `self.CapsuleComponent.OnComponentBeginOverlap`
  (params (OverlappedComponent :type "PrimitiveComponent Object Reference") (OtherActor :type "Actor Object Reference") (OtherComp :type "PrimitiveComponent Object Reference") (OtherBodyIndex :type Integer) (bFromSweep :type Boolean) (SweepResult :type "HitResult Structure (by ref)"))
  (`self.KillOrDefeatByEnemy` OtherActor OtherActor))

(event `self.OnWalkingOffLedge`
  (params (PreviousFloorImpactNormal :type "Vector Structure (by ref)") (PreviousFloorContactNormal :type "Vector Structure (by ref)") (PreviousLocation :type "Vector Structure (by ref)") (TimeDelta :type "Float (single-precision)"))
  (set `self.IsInCayoteTime` true)
  (`KismetSystemLibrary.RetriggerableDelay` (`self.CayoteTime`))
  (set `self.IsInCayoteTime` false))

(fn `CallRestartPlayer`
  (locals (ControllerRef :type "Controller Object Reference"))
  (bind _returnvalue (`GameplayStatics.GetPlayerController` (`self.index`)))
  (bind _output_get (set `local.ControllerRef` (`self.GetController`)))
  (bind _asplayer_controller (cast `PlayerController` _output_get))
  (bind _output_get_2 (set `self.index` (`GameplayStatics.GetPlayerControllerID` _asplayer_controller)))
  (if (== _output_get_2 0)
    (bind _outactors (`GameplayStatics.GetAllActorsWithTag` "Start1"))
    (for _array_element _outactors
      (bind _returnvalue_2 (pcsubsystem `EnhancedInputLocalPlayerSubsystem` _asplayer_controller))
      (message `EnhancedInputSubsystemInterface.AddMappingContext` _returnvalue_2 "/Game/Input/Hero_ZD_Mapping.Hero_ZD_Mapping" 0 (struct))
      (`self.K2_DestroyActor`)
      (cast `/Game/Blueprints/GameMode_Platform` (`GameplayStatics.GetGameMode`))
      (bind _returnvalue_3 (`|SpawnActorFromClass` "BP_Boy_ZD_C" (`self.GetTransform` _array_element) "Undefined" "MultiplyWithRoot" null null))
      (`Controller.Possess` _returnvalue _returnvalue_3))
    (else
      (bind _outactors_2 (`GameplayStatics.GetAllActorsWithTag` "Start2"))
      (for _array_element_2 _outactors_2
        (message `EnhancedInputSubsystemInterface.AddMappingContext` _returnvalue_2 "/Game/Input/Hero_ZD_Mapping2.Hero_ZD_Mapping2" 0 (struct))
        (`self.K2_DestroyActor`)
        (cast `/Game/Blueprints/GameMode_Platform` (`GameplayStatics.GetGameMode`))
        (bind _returnvalue_4 (`|SpawnActorFromClass` "BP_Boy_ZD_C" (`self.GetTransform` _array_element_2) "Undefined" "MultiplyWithRoot" null null))
        (`Controller.Possess` _returnvalue _returnvalue_4)))))

(fn `CanJumpInternal`
  (returns (ReturnValue :type Boolean))
  (bind _returnvalue (`parent.CanJumpInternal`))
  (return (or _returnvalue (`self.IsInCayoteTime`))))

(fn `DefeatEffect`
  (bind _asplayer_controller (cast `PlayerController` (`self.GetController`)))
  (if (== (`GameplayStatics.GetPlayerControllerID` _asplayer_controller) 0)
    (bind _returnvalue (pcsubsystem `EnhancedInputLocalPlayerSubsystem` _asplayer_controller))
    (`EnhancedInputSubsystemInterface.RemoveMappingContext` _returnvalue "/Game/Input/Hero_ZD_Mapping.Hero_ZD_Mapping" (struct))
    (`SceneComponent.K2_DetachFromComponent` (`self.SpringArm`) "KeepWorld" "KeepWorld" "KeepWorld" true)
    (`GameplayStatics.PlayWorldCameraShake` "/Game/CameraShake/CS_Def.CS_Def_C" (`self.K2_GetActorLocation`) 0.0 10000.0 0.0)
    (else
      (`EnhancedInputSubsystemInterface.RemoveMappingContext` _returnvalue "/Game/Input/Hero_ZD_Mapping2.Hero_ZD_Mapping2" (struct))
      (`SceneComponent.K2_DetachFromComponent` (`self.SpringArm`) "KeepWorld" "KeepWorld" "KeepWorld" true)
      (`GameplayStatics.PlayWorldCameraShake` "/Game/CameraShake/CS_Def.CS_Def_C" (`self.K2_GetActorLocation`) 0.0 10000.0 0.0))))

(fn `KillOrDefeatByEnemy`
  (params (Object :type "Object Object Reference") (Object2 :type "Object Object Reference"))
  (bind (_returnvalue_x _returnvalue_y _returnvalue_z) (`KismetMathLibrary.BreakVector` (`self.GetVelocity`)))
  (bind (_returnvalue_x_2 _returnvalue_y_2 _returnvalue_z_2) (`KismetMathLibrary.BreakVector` (`self.GetVelocity`)))
  (`|ExecutionSequence`
    (:`then_0`
      (bind _asbp_bat_zd (cast `/Game/Blueprints/Characters/Bat/BP_Bat_ZD` Object))
      (if (and (`NavMovementComponent.IsFalling` (`self.CharacterMovement`)) (< _returnvalue_z 0.0))
        (`self.Defead` _asbp_bat_zd)
        (`self.LaunchCharacter` (`KismetMathLibrary.MakeVector` 0.0 0.0 (`self.Enemy Bounce Launch`)))
        (else
          (`self.Defead`)
          (`GameplayStatics.PlaySound2D` "/Game/Sounds/kill_by_bat.kill_by_bat" 1.0 1.0 0.0 null null))))
    (:`then_1`
      (bind _asbp_rat_zd (cast `/Game/Blueprints/Characters/Rat/BP_Rat_ZD` Object2))
      (if (and (`NavMovementComponent.IsFalling` (`self.CharacterMovement`)) (< _returnvalue_z_2 0.0))
        (`self.Defead` _asbp_rat_zd)
        (`self.LaunchCharacter` (`KismetMathLibrary.MakeVector` 0.0 0.0 (`self.Enemy Bounce Launch`)))
        (else
          (`self.Defead`)
          (`GameplayStatics.PlaySound2D` "/Game/Sounds/died_Cue.died_Cue" 1.0 1.0 0.0 null null))))))

(fn `Trace for Platforms`
  (bind _returnvalue (`SceneComponent.K2_GetComponentLocation` (`self.FootPosition`)))
  (if (`NavMovementComponent.IsFalling` (`self.CharacterMovement`))
    (bind (_outhit _returnvalue_2) (`KismetSystemLibrary.LineTraceSingleForObjects` :`Start` _returnvalue :`End` (+ _returnvalue (* (`KismetMathLibrary.Vector_Down`) (`self.PlatformCheckDistance`))) :`ObjectTypes` (`|MakeArray` "ObjectTypeQuery7" :!type "EObjectTypeQuery Enum") :`DrawDebugType` "ForOneFrame"))
    (if _returnvalue_2
      (`PrimitiveComponent.SetCollisionResponseToChannel` (`self.CapsuleComponent`) "ECC_GameTraceChannel1" "ECR_Block")
      (else
        (`PrimitiveComponent.SetCollisionResponseToChannel` (`self.CapsuleComponent`) "ECC_GameTraceChannel1" "ECR_Overlap")))))

(fn `UpdateContollerRotation`
  (bind _returnvalue (`self.GetController`))
  (bind _returnvalue_2 (`self.GetController`))
  (bind _velocity_x (`KismetMathLibrary.BreakVector` (`MovementComponent.Velocity` (`self.CharacterMovement`))))
  (`/Engine/EditorBlueprintResources/StandardMacros.CompareFloat` _velocity_x
    (:`>`
      (`/Engine/EditorBlueprintResources/StandardMacros.IsValid` _returnvalue_2
        (:`Is Valid`
          (`Controller.SetControlRotation` _returnvalue_2 (`KismetMathLibrary.MakeRotator` 0.0)))))
    (:`<`
      (`/Engine/EditorBlueprintResources/StandardMacros.IsValid` _returnvalue
        (:`Is Valid`
          (`Controller.SetControlRotation` _returnvalue (`KismetMathLibrary.MakeRotator` 0.0 0.0 180.0)))))))

(fn `UserConstructionScript`
  (`parent.UserConstructionScript`))