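; BP_Goal_Poppy is a poppy level goal that the boy character collects to win.
; When BP_Boy_ZD first overlaps its Box, a DoOnce calls TriggerGaol to swap the Paper2D sprite to the taken variant and prints a Polish win message.
; After a short delay it reopens the current level by name, so winning restarts the same level rather than advancing.
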(event `self.Box.OnComponentBeginOverlap`
  (params (OverlappedComponent :type "PrimitiveComponent Object Reference") (OtherActor :type "Actor Object Reference") (OtherComp :type "PrimitiveComponent Object Reference") (OtherBodyIndex :type Integer) (bFromSweep :type Boolean) (SweepResult :type "HitResult Structure (by ref)"))
  (cast `/Game/Blueprints/Characters/Boy/BP_Boy_ZD` OtherActor)
  (`/Engine/EditorBlueprintResources/StandardMacros.DoOnce` false
    (:`Completed`
      (`self.TriggerGaol`)
      (`KismetSystemLibrary.PrintString` "Wygrales")
      (bind _returnvalue (`GameplayStatics.GetCurrentLevelName` true))
      (`KismetSystemLibrary.Delay` 3.0)
      (`GameplayStatics.OpenLevel` (`KismetStringLibrary.Conv_StringToName` _returnvalue)))))

(fn `TriggerGaol`
  (`PaperSpriteComponent.SetSprite` (`self.PaperSprite`) "/Game/Sprites/Enviroment/Poppy/Poppy_Taken_Sprite.Poppy_Taken_Sprite"))

(fn `UserConstructionScript`)